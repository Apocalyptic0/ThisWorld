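; BP_Beam is a sprite beam element that shoots from its instigating Paper character toward the mouse cursor in the XZ plane, or bounces off mirrors.
; Each Tick it re-aims, line-traces to the first hit, stretches its X scale to that distance and debug-draws the endpoint.
; Reflection beams start at their Source beam's endpoint, mirror its direction about the BP_Mirror normal, and self-destroy when Source is invalid.
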(event `self.ReceiveBeginPlay`)

(event `self.ReceiveTick`
  (params (DeltaSeconds :type "Float (single-precision)"))
  (`|ExecutionSequence`
    (:`then_0`
      (bind _asbp_stextra_paper_character (cast `/Game/Player/BP_STExtraPaperCharacter` (`self.ElementInstigator`)))
      (set `self.StartPoint` (`self.K2_GetActorLocation` _asbp_stextra_paper_character))
      (set `self.Direction` (`KismetMathLibrary.Normal` (`KismetMathLibrary.MakeVector` (.x (- (`PlayerController.DeprojectMousePositionToWorld` (`GameplayStatics.GetPlayerController` 0)) (`self.StartPoint`))) 0.0 (.z (- (`PlayerController.DeprojectMousePositionToWorld` (`GameplayStatics.GetPlayerController` 0)) (`self.StartPoint`))))))
      (`self.SetTransform`))
    (:`then_1`
      (if (`self.bReflection`)
        (if (`KismetSystemLibrary.IsValid` (`self.Source`))
          (set `self.StartPoint` (`/Game/Actors/Elements/BP_Beam.ActuallyEndPoint` (`self.Source`)))
          (`self.GetReflectDirection`)
          (`self.SetTransform`)
          (else
            (`self.K2_DestroyActor`)))))))

(fn `CalculateBeamLengthWithCollision`
  (returns (Length :type "Float (double-precision)"))
  (bind (_outhit _returnvalue) (`KismetSystemLibrary.LineTraceSingle` (`self.StartPoint`) (`self.EndPoint`) "TraceTypeQuery1" false (`|MakeArray` (`self.ElementInstigator`))))
  (if _returnvalue
    (return (`.Distance` (`GameplayStatics.BreakHitResult` _outhit)))
    (else
      (return (`self.Length`)))))

(fn `GetReflectDirection`
  (bind _direction (`/Game/Actors/Elements/BP_Beam.Direction` (`self.Source`)))
  ; 后面换Interface
  (bind _asbp_mirror (cast `/Game/Actors/InteractiveActors/BP_Mirror` (`self.ReflectedActor`)))
  (bind _returnvalue (`KismetMathLibrary.Normal` (`/Game/Actors/InteractiveActors/BP_Mirror.NormalDir` _asbp_mirror)))
  (set `self.Direction` (- _direction (* (* (`KismetMathLibrary.Dot_VectorVector` _direction _returnvalue) 2.0) _returnvalue))))

(fn `SetTransform`
  (set `self.EndPoint` (+ (`self.StartPoint`) (* (`self.Direction`) (`self.Length`))))
  (`self.K2_SetActorLocationAndRotation` (`self.StartPoint`) (`KismetMathLibrary.Conv_VectorToRotator` (`self.Direction`)))
  (bind _length (`self.CalculateBeamLengthWithCollision`))
  (`self.SetActorScale3D` (`KismetMathLibrary.MakeVector` (/ _length (`self.OriginSpriteSize`)) 1.0 1.0))
  (bind _output_get (set `self.ActuallyEndPoint` (+ (`self.StartPoint`) (* (`self.Direction`) _length))))
  (`KismetSystemLibrary.DrawDebugCircle` _output_get 5.0 12 (struct :`R` 1.0 :`G` 1.0 :`B` 1.0 :`A` 1.0) 10.0 1.0))

(fn `UserConstructionScript`)