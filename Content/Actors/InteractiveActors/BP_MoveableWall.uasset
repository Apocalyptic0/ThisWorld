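; BP_MoveableWall is an interactive wall actor that rises in steps and then removes itself.
; On BeginPlay it binds its move event through BindEventToMoveAndDestroy, so an external trigger can start it.
; The move event starts a looping one-second timer that nudges the wall upward and increments a counter.
; When the counter reaches five, the timer is cleared and the actor is destroyed.
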(event `self.ReceiveBeginPlay`
  (add `self.MoveAndDestroy` (delegate `MoveEvent`)))

(event `MoveEvent`
  (bind _returnvalue (`KismetSystemLibrary.K2_SetTimerDelegate` (delegate `MoveTimerEvent`) 1.0 true))
  (set `self.MoveTimerHandle` _returnvalue))

(event `MoveTimerEvent`
  (`self.K2_SetActorLocation` (+ (`self.K2_GetActorLocation`) (0.0 0.0 20.0)))
  (bind _result (`/Engine/EditorBlueprintResources/StandardMacros.IncrementInt` (`self.Count`))
    (:`  `
      (if (== _result 5)
        (`KismetSystemLibrary.K2_ClearAndInvalidateTimerHandle` (`self.MoveTimerHandle`))
        (`self.K2_DestroyActor`)))))

(fn `UserConstructionScript`)