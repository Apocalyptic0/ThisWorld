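; BP_Mirror is an interactive mirror actor that reflects BP_Beam actors.
; On begin play it computes a facing normal in the XZ plane from its rotation plus an origin offset.
; Overlapping beams that face the normal, were not instigated by this mirror and pass an element bitmask check replace any existing reflection with a new spawned BP_Beam linked to the source and mirror.
; Ending an overlap destroys the reflected beam.
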(event `self.ReceiveBeginPlay`
  (bind _output_get (set `self.NormalDir` (`KismetMathLibrary.MakeVector` (.x (`KismetMathLibrary.Conv_RotatorToVector` (`KismetMathLibrary.ComposeRotators` (`self.K2_GetActorRotation` self) (`self.NormalOriginRotator`)))) 0.0 (.z (`KismetMathLibrary.Conv_RotatorToVector` (`KismetMathLibrary.ComposeRotators` (`self.K2_GetActorRotation` self) (`self.NormalOriginRotator`))))))))

(event `self.RenderComponent.OnComponentBeginOverlap`
  (params (OverlappedComponent :type "PrimitiveComponent Object Reference") (OtherActor :type "Actor Object Reference") (OtherComp :type "PrimitiveComponent Object Reference") (OtherBodyIndex :type Integer) (bFromSweep :type Boolean) (SweepResult :type "HitResult Structure (by ref)"))
  (bind _asbp_beam (cast `/Game/Actors/Elements/BP_Beam` OtherActor))
  (if (and (!= (`ElementPaperActorBase.ElementInstigator` _asbp_beam) self) (< (`KismetMathLibrary.Dot_VectorVector` (`/Game/Actors/Elements/BP_Beam.Direction` _asbp_beam) (`self.NormalDir`)) 0.0))
    (`self.OnAbsorbingElement` _asbp_beam)))

(event `self.RenderComponent.OnComponentEndOverlap`
  (params (OverlappedComponent :type "PrimitiveComponent Object Reference") (OtherActor :type "Actor Object Reference") (OtherComp :type "PrimitiveComponent Object Reference") (OtherBodyIndex :type Integer))
  (bind _reflectedbeam (`self.ReflectedBeam`))
  (if (`KismetSystemLibrary.IsValid` _reflectedbeam)
    (`self.K2_DestroyActor` _reflectedbeam)))

(event `self.OnAbsorbingElement`
  (params (ElementActor :type "ElementPaperActorBase Object Reference"))
  (bind _returnvalue (`ElementPaperActorBase.HasElements` ElementActor (`KismetMathLibrary.Conv_IntToByte` (`|BitmaskLiteral` 1))))
  (if _returnvalue
    (`self.GenerateElement` ElementActor)))

(fn `GenerateElement`
  (params (ElementActor :type "ElementPaperActorBase Object Reference"))
  (returns (ReturnValue :type "ElementPaperActorBase Object Reference"))
  (bind _reflectedbeam (`self.ReflectedBeam`))
  (`|ExecutionSequence`
    (:`then_0`
      (if (`KismetSystemLibrary.IsValid` _reflectedbeam)
        (`self.K2_DestroyActor` _reflectedbeam)))
    (:`then_1`
      (bind _asbp_beam (cast `/Game/Actors/Elements/BP_Beam` ElementActor)
        (:`then`
          (bind _returnvalue (`|SpawnActorFromClass` "/Game/Actors/Elements/BP_Beam.BP_Beam_C" (`KismetMathLibrary.MakeTransform` (0.0 0.0 0.0)) "Undefined" "MultiplyWithRoot" null null))
          (set `/Game/Actors/Elements/BP_Beam.Source` _asbp_beam _returnvalue)
          (set `/Game/Actors/Elements/BP_Beam.bReflection` true _returnvalue)
          (set `/Game/Actors/Elements/BP_Beam.ReflectedActor` self _returnvalue)
          (set `ElementPaperActorBase.ElementInstigator` self _returnvalue)
          (set `self.ReflectedBeam` _returnvalue))
        (:`CastFailed`
          (return null))))))

(fn `UserConstructionScript`)