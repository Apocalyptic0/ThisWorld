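; Interactive water container that rises in steps when it absorbs a matching element, simulating filling.
; Overlap of its render component with a BP_Water actor triggers OnAbsorbingElement, which checks that actor's element bitmask.
; A match starts a looping one-second timer, unless one is already valid, that teleports the whole actor upward without sweep.
; A counter clears the timer after five steps and resets, so later absorptions raise it again.
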(event `self.OnAbsorbingElement`
  (params (ElementActor :type "ElementPaperActorBase Object Reference"))
  (bind _returnvalue (`ElementPaperActorBase.HasElements` ElementActor (`KismetMathLibrary.Conv_IntToByte` (`|BitmaskLiteral` 2))))
  (if _returnvalue
    (if (not (`KismetSystemLibrary.K2_IsValidTimerHandle` (`self.FillWaterTimer`)))
      (bind _returnvalue_2 (`KismetSystemLibrary.K2_SetTimerDelegate` (delegate `FillWater`) 1.0 true))
      (set `self.FillWaterTimer` _returnvalue_2))))

(event `FillWater`
  (`self.K2_SetActorLocation` (+ (`self.K2_GetActorLocation`) (0.0 0.0 20.0)))
  (bind _result (`/Engine/EditorBlueprintResources/StandardMacros.IncrementInt` (`self.Count`))
    (:`  `
      (if (== _result 5)
        (set `self.Count` 0)
        (`KismetSystemLibrary.K2_ClearAndInvalidateTimerHandle` (`self.FillWaterTimer`))))))

(event `self.RenderComponent.OnComponentBeginOverlap`
  (params (OverlappedComponent :type "PrimitiveComponent Object Reference") (OtherActor :type "Actor Object Reference") (OtherComp :type "PrimitiveComponent Object Reference") (OtherBodyIndex :type Integer) (bFromSweep :type Boolean) (SweepResult :type "HitResult Structure (by ref)"))
  (bind _asbp_water (cast `/Game/Actors/Elements/BP_Water` OtherActor))
  (`self.OnAbsorbingElement` _asbp_water))

(fn `UserConstructionScript`)