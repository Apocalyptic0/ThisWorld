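; Player controller for the 2D Paper character that turns Enhanced Input into movement and creates the player HUD.
; On BeginPlay it adds the input mapping context, caches the character and puts WBP_PlayerUI on screen.
; Move input drives horizontal movement, crouching on down, climbing on up when CanClimb is set, and flips the sprite by X velocity.
; Jump input triggers a jump only when the character can jump and CanClimb is off.
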(event `self.ReceiveBeginPlay`
  (bind _returnvalue (pcsubsystem `EnhancedInputLocalPlayerSubsystem` self))
  (if (`KismetSystemLibrary.IsValid` _returnvalue)
    (`EnhancedInputSubsystemInterface.AddMappingContext` _returnvalue "/Game/Player/Inputs/IM_PaperCharacter.IM_PaperCharacter" 0 (struct))
    (bind _asbp_stextra_paper_character (cast `/Game/Player/BP_STExtraPaperCharacter` (`GameplayStatics.GetPlayerCharacter` 0)))
    (set `self.Paper Character` _asbp_stextra_paper_character)
    (bind _returnvalue_2 (`|CreateWidget` "/Game/UI/WBP_PlayerUI.WBP_PlayerUI_C"))
    (bind _output_get (set `self.PlayerUI` _returnvalue_2))
    (`UserWidget.AddToViewport` _output_get 0)))

(event `EnhancedInput|/Game/Player/Inputs/IA_Move`
  (params (ActionValue :type "Vector2D Structure") (ElapsedSeconds :type "Float (double-precision)") (TriggeredSeconds :type "Float (double-precision)") (InputAction :type "InputAction Object Reference" :default "/Game/Player/Inputs/IA_Move.IA_Move"))
  (bind (_x _y) (`KismetMathLibrary.BreakVector2D` ActionValue))
  (bind _paper_character (`self.Paper Character`))
  (bind _paper_character_2 (`self.Paper Character`))
  (bind _paper_character_3 (`self.Paper Character`))
  (bind _sprite (`PaperCharacter.Sprite` _paper_character_3))
  (:`Triggered`
    (`Pawn.AddMovementInput` _paper_character (`KismetMathLibrary.GetForwardVector` (`self.GetControlRotation`)) _x false)
    (`|ExecutionSequence`
      (:`then_0`
        (if (and (`Character.CanCrouch` _paper_character) (== _y -1.0))
          (`Character.Crouch` (`self.Paper Character`))))
      (:`then_1`
        (if (>= (.x (`self.GetVelocity` _paper_character_3)) 0.0)
          (`SceneComponent.K2_SetRelativeRotation` :`self` _sprite)
          (else
            (`SceneComponent.K2_SetRelativeRotation` _sprite (struct :`Yaw` -180.0) false false))))
      (:`then_2`
        (if (and (> _y 0.0) (`STExtraPaperCharacter.bCanClimb` _paper_character_2))
          (`Pawn.AddMovementInput` _paper_character_2 (`KismetMathLibrary.GetUpVector` (`self.GetControlRotation`)) _y false))))))

(event `EnhancedInput|/Game/Player/Inputs/IA_Jump`
  (params (ActionValue :type Boolean) (ElapsedSeconds :type "Float (double-precision)") (TriggeredSeconds :type "Float (double-precision)") (InputAction :type "InputAction Object Reference" :default "/Game/Player/Inputs/IA_Jump.IA_Jump"))
  (:`Triggered`
    (bind _asbp_stextra_paper_character (cast `/Game/Player/BP_STExtraPaperCharacter` (`GameplayStatics.GetPlayerCharacter` 0)))
    (if (and (`Character.CanJump` _asbp_stextra_paper_character) (not (`STExtraPaperCharacter.bCanClimb` _asbp_stextra_paper_character)))
      (`Character.Jump` _asbp_stextra_paper_character))))

(fn `UserConstructionScript`)