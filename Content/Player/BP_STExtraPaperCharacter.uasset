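; Player Paper2D character that switches between five elements, casts elemental skills and reveals elements on interactive actors.
; Number keys set EnergyType and recolor the controller's UI energy ring, whose percent also stores the energy value.
; Left click spawns Light or Water skills from OwningSkills, draining energy without checking it; Q refills, and middle click reveals Light actors only.
; Jump, ledge-fall and landing events jump animation state nodes directly.
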(event `Key|Q`
  (params (Key :type "Key Structure"))
  ; TODO：吸收能量/回收技能
  (:`Pressed`
    (`self.AddEnergyPercent` 10.0)))

(event `Key|MiddleMouseButton`
  (params (Key :type "Key Structure"))
  ; TODO：元素视野
  (:`Pressed`
    (bind _outactors (`GameplayStatics.GetAllActorsOfClass` "/Script/ThisWorld.Element_InteractiveActorBase"))
    (for _array_element _outactors
      (switch `EMyElementType` (`Element_InteractiveActorBase.MainInteractiveElement` _array_element)
        (:`Light`
          (`Element_InteractiveActorBase.ShowMainInteractiveElement` _array_element))))))

(event `Key|Three`
  (params (Key :type "Key Structure"))
  ; 切换元素类型
  (:`Pressed`
    (bind _output_get (set `self.EnergyType` "Fire"))
    (`self.ChangeEnergyType` _output_get)))

(event `Key|Five`
  (params (Key :type "Key Structure"))
  ; 切换元素类型
  (:`Pressed`
    (bind _output_get (set `self.EnergyType` "Electricity"))
    (`self.ChangeEnergyType` _output_get)))

(event `Key|One`
  (params (Key :type "Key Structure"))
  ; 切换元素类型
  (:`Pressed`
    (bind _output_get (set `self.EnergyType` "Light"))
    (`self.ChangeEnergyType` _output_get)))

(event `Key|Two`
  (params (Key :type "Key Structure"))
  ; 切换元素类型
  (:`Pressed`
    (bind _output_get (set `self.EnergyType` "Water"))
    (`self.ChangeEnergyType` _output_get)))

(event `Key|Four`
  (params (Key :type "Key Structure"))
  ; 切换元素类型
  (:`Pressed`
    (bind _output_get (set `self.EnergyType` "Wind"))
    (`self.ChangeEnergyType` _output_get)))

(event `Key|LeftMouseButton`
  (params (Key :type "Key Structure"))
  (bind _owningskills (`self.OwningSkills`))
  ; TODO：释放技能
  (:`Pressed`
    (switch `EMyElementType` (`self.EnergyType`)
      (:`Light`
        (bind _returnvalue (`|SpawnActorFromClass` (`BlueprintMapLibrary.Map_Find` _owningskills "Beam") (`KismetMathLibrary.MakeTransform` (0.0 0.0 0.0)) "AlwaysSpawn" "MultiplyWithRoot" null null))
        (`self.UseSkill` _returnvalue)
        (`self.AddEnergyPercent` -10.0))
      (:`Water`
        (bind _returnvalue_2 (`|SpawnActorFromClass` (`BlueprintMapLibrary.Map_Find` _owningskills "Water") (`KismetMathLibrary.MakeTransform` (0.0 0.0 0.0)) "AlwaysSpawn" "MultiplyWithRoot" null null))
        (`self.UseSkill` _returnvalue_2)
        (`self.AddEnergyPercent` -10.0)))))

(event `self.OnJumped`
  (`PaperZDAnimInstance.JumpToNode` (`PaperZDAnimationComponent.AnimInstance` (`self.AnimationComponent`)) "JumpState" "None"))

(event `self.OnWalkingOffLedge`
  (params (PreviousFloorImpactNormal :type "Vector Structure (by ref)") (PreviousFloorContactNormal :type "Vector Structure (by ref)") (PreviousLocation :type "Vector Structure (by ref)") (TimeDelta :type "Float (single-precision)"))
  (`PaperZDAnimInstance.JumpToNode` (`PaperZDAnimationComponent.AnimInstance` (`self.AnimationComponent`)) "FallingState" "None"))

(event `self.OnLanded`
  (params (Hit :type "HitResult Structure (by ref)"))
  (`PaperZDAnimInstance.JumpToNode` (`PaperZDAnimationComponent.AnimInstance` (`self.AnimationComponent`)) "LandState" "None"))

(fn `AddEnergyPercent`
  (params (val :type "Float (double-precision)"))
  (bind _asbp_stextra_paper_character_controller (cast `/Game/Player/BP_STExtraPaperCharacterController` (`self.GetController`)))
  (bind _wbp_ringenergy (`/Game/UI/WBP_PlayerUI.WBP_RingEnergy` (`/Game/Player/BP_STExtraPaperCharacterController.PlayerUI` _asbp_stextra_paper_character_controller)))
  (`/Game/UI/WBP_RingEnergy.SetPercent` _wbp_ringenergy (`KismetMathLibrary.FClamp` (+ (`/Game/UI/WBP_RingEnergy.Percent` _wbp_ringenergy) (/ val 100.0)))))

(fn `ChangeEnergyType`
  (params (EnergyType :type "EMyElementType Enum" :default "Null"))
  (locals (Color :type "LinearColor Structure" :default (struct :`A` 1.0)))
  (bind _asbp_stextra_paper_character_controller (cast `/Game/Player/BP_STExtraPaperCharacterController` (`self.GetController`)))
  (switch `EMyElementType` EnergyType
    (:`Light`
      (set `local.Color` (struct :`R` 1.0 :`G` 0.71167 :`A` 1.0)))
    (:`Water`
      (set `local.Color` (struct :`G` 0.046114 :`B` 1.0 :`A` 1.0)))
    (:`Fire`
      (set `local.Color` (struct :`R` 0.657986 :`G` 0.019488 :`A` 1.0)))
    (:`Wind`
      (set `local.Color` (struct :`R` 0.041871 :`G` 1.0 :`A` 1.0)))
    (:`Electricity`
      (set `local.Color` (struct :`R` 0.839691 :`G` 1.0 :`A` 1.0))))
  (set `UserWidget.ColorAndOpacity` (`local.Color`) (`/Game/UI/WBP_PlayerUI.WBP_RingEnergy` (`/Game/Player/BP_STExtraPaperCharacterController.PlayerUI` _asbp_stextra_paper_character_controller))))

(fn `UserConstructionScript`)